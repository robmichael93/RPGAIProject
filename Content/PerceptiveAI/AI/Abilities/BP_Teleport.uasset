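; BP_Teleport is an AI ability actor that teleports its owner to a location chosen by the Environment Query System.
; On BeginPlay it runs EQS_TeleportQuery with the owner as querier, picking randomly from the best 5% of results.
; When the query finishes with valid locations, it moves the owner to the first one with a zeroed rotation.
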(event `self.ReceiveBeginPlay`
  (`parent.ReceiveBeginPlay`)
  (`KismetSystemLibrary.PrintString` "Activating Teleport" true true (struct :`G` 0.66 :`B` 1.0 :`A` 1.0) 10.0)
  (bind _returnvalue (`EnvQueryManager.RunEQSQuery` "/Game/PerceptiveAI/AI/EQS/EQS_TeleportQuery.EQS_TeleportQuery" (`self.GetOwner`) "RandomBest5Pct"))
  (add `EnvQueryInstanceBlueprintWrapper.OnQueryFinishedEvent` _returnvalue (`|CreateDelegate` :!event `OnQueryFinished`)))

(event `OnQueryFinished`
  (params (QueryInstance :type "EnvQueryInstanceBlueprintWrapper Object Reference") (QueryStatus :type "EEnvQueryStatus Enum" :default "Processing"))
  (bind (_resultlocations _returnvalue) (`EnvQueryInstanceBlueprintWrapper.GetQueryResultsAsLocations` QueryInstance))
  (if _returnvalue
    (`self.K2_TeleportTo` :`self` (`self.GetOwner`) :`DestLocation` (`|GetArrayItem` _resultlocations))))

(fn `UserConstructionScript`
  (`parent.UserConstructionScript`))